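; Futuristic soldier character Blueprint that handles quick construction and the on-screen balance (disbalance) bar.
; Quick construct passes the PlayerHUD's selected item to TryConstruct, and key 9 drops an energy pack.
; Balance UI lives here rather than in C++: a widget shows PlayerState balance while a looping timer steps it by -1, and both are cleared at its limits.
; Leftover debug code prints whether a "TEST"-tagged actor is in front or behind every tick.
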(event `self.ReceiveBeginPlay`
  (bind _outactors (`GameplayStatics.GetAllActorsWithTag` "TEST"))
  (set `self.Delthis` (`|GetArrayItem` _outactors)))

(event `self.ReceiveTick`
  (params (DeltaSeconds :type "Float (single-precision)"))
  (if (< (`KismetMathLibrary.Dot_VectorVector` (`self.GetActorForwardVector`) (- (`self.K2_GetActorLocation` (`self.Delthis`)) (`self.K2_GetActorLocation`))) 0.0)
    (`KismetSystemLibrary.PrintString` "behind")
    (else
      (`KismetSystemLibrary.PrintString` "infront"))))

(event `self.TryQuickConstruct`
  (bind _mycontroller (`self.myController`))
  (`/Engine/EditorBlueprintResources/StandardMacros.IsValid` _mycontroller
    (:`Is Valid`
      (bind _asplayer_hud (cast `/Game/UI/HUD/PlayerHUD` (`PlayerController.GetHUD` _mycontroller)))
      (bind _selectedconstruct (`/Game/UI/HUD/PlayerHUD.GetCurrentSelectedConstructed` _asplayer_hud))
      (`self.TryConstruct` _selectedconstruct))))

(event `Key|Nine`
  (params (Key :type "Key Structure"))
  (:`Pressed`
    (`self.DropEnergyPack`)))

(event `Key|Eight`
  (params (Key :type "Key Structure"))
  (:`Pressed`
    (`KismetSystemLibrary.PrintString` "Hello")))

(event `self.HUD_ShowDisbalanceBar`
  (bind _myplayerstate (`self.myPlayerState`))
  (bind _balance (`ShooterSandboxPlayerState.balance` _myplayerstate))
  ;[0.1389 1 0.5027] Balance Stuff - Done here to avoid needless complexity and a bunch of functions in C++ that won't be useful in other mechanics anyway
  (`/Engine/EditorBlueprintResources/StandardMacros.IsValid` (`self.myPlayerState`)
    (:`Is Valid`
      (if (not (`self.BALANCE_balanceWidgetOn`))
        (bind _returnvalue (`|CreateWidget` "/Game/UI/Balance.Balance_C" (`GameplayStatics.GetPlayerController` 0)))
        (bind _output_get (set `self.BalanceScreen` _returnvalue))
        (`UserWidget.AddToViewport` _output_get 0)
        (set `self.BALANCE_balanceWidgetOn` true))
      (`/Game/UI/Balance.SetBalanceBarValue` (`self.BalanceScreen`) (/ (`KismetMathLibrary.Conv_IntToDouble` _balance) (* (`KismetMathLibrary.Conv_IntToDouble` (`ShooterSandboxPlayerState.currentMaxBalance` _myplayerstate)) 2.0)))
      (if (<= _balance 0)
        (`self.Client_RemoveBalance`)
        (elif (not (`KismetSystemLibrary.K2_IsValidTimerHandle` (`self.BALANCE_regenTimer`)))
          (bind _returnvalue_2 (`KismetSystemLibrary.K2_SetTimerDelegate` (delegate `RegenBalance`) 0.1 true))
          (set `self.BALANCE_regenTimer` _returnvalue_2))))))

(event `RegenBalance`
  (bind _myplayerstate (`self.myPlayerState`))
  ;[0.1389 1 0.5027] Balance Stuff - Done here to avoid needless complexity and a bunch of functions in C++ that won't be useful in other mechanics anyway
  (bind _returnvalue (`ShooterSandboxPlayerState.BalanceChangedBy` _myplayerstate -1))
  (if (>= _returnvalue (`ShooterSandboxPlayerState.currentMaxBalance` _myplayerstate))
    (`self.Client_RemoveBalance`)
    (else
      (`self.Client_DisbalanceBar`))))

(event `Client_RemoveBalance`
  ;[0.1389 1 0.5027] Balance Stuff - Done here to avoid needless complexity and a bunch of functions in C++ that won't be useful in other mechanics anyway
  (`KismetSystemLibrary.K2_ClearAndInvalidateTimerHandle` (`self.BALANCE_regenTimer`))
  (`Widget.RemoveFromParent` (`self.BalanceScreen`))
  (set `self.BALANCE_balanceWidgetOn` false))

(fn `UserConstructionScript`)