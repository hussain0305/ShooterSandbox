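; BPWC_SwingBar is a swing bar actor that shows a widget while a ShooterSandboxCharacter is within its Sphere trigger.
; The widget is hidden on BeginPlay, and Sphere begin and end overlaps toggle it through the WidgetVisibility event.
; Each overlap also prints an availability message; the graph contains no swing logic itself.
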(event `WidgetVisibility`
  (params (Visibility :type Boolean))
  (`SceneComponent.SetVisibility` (`self.Widget`) Visibility false))

(event `self.ReceiveBeginPlay`
  (`self.WidgetVisibility` false))

(event `self.Sphere.OnComponentBeginOverlap`
  (params (OverlappedComponent :type "PrimitiveComponent Object Reference") (OtherActor :type "Actor Object Reference") (OtherComp :type "PrimitiveComponent Object Reference") (OtherBodyIndex :type Integer) (bFromSweep :type Boolean) (SweepResult :type "HitResult Structure (by ref)"))
  (bind _asshooter_sandbox_character (cast `ShooterSandboxCharacter` OtherActor))
  (`/Engine/EditorBlueprintResources/StandardMacros.IsValid` _asshooter_sandbox_character
    (:`Is Valid`
      (`KismetSystemLibrary.PrintString` "Bar swing available")
      (`self.WidgetVisibility` true))))

(event `self.Sphere.OnComponentEndOverlap`
  (params (OverlappedComponent :type "PrimitiveComponent Object Reference") (OtherActor :type "Actor Object Reference") (OtherComp :type "PrimitiveComponent Object Reference") (OtherBodyIndex :type Integer))
  (bind _asshooter_sandbox_character (cast `ShooterSandboxCharacter` OtherActor))
  (`/Engine/EditorBlueprintResources/StandardMacros.IsValid` _asshooter_sandbox_character
    (:`Is Valid`
      (`KismetSystemLibrary.PrintString` "Bar swing unavailable")
      (`self.WidgetVisibility` false))))

(fn `UserConstructionScript`)