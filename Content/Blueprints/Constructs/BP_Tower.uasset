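; Tower actor with a shield, a lift and four directional triggers that spawn platforms, all reacting to ShooterSandboxCharacter overlaps.
; A looping timer eases the shield's Y scale to a quarter while characters are in Vicinity, restoring it when their count drops below one.
; LiftPad plays and reverses a timeline that moves TowerLift.
; Each platform trigger, on authority only, spawns a ChainPlatform ahead of itself, unless collision blocks it.
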(event `self.ReceiveBeginPlay`
  (bind _output_get (set `self.ShieldOriginalHeight` (.y (`SceneComponent.K2_GetComponentScale` (`self.TowerShield`)))))
  (set `self.ShieldShrunkHeight` (/ _output_get 4.0)))

(event `self.ReceiveTick`
  (params (DeltaSeconds :type "Float (single-precision)")))

(event `self.Vicinity.OnComponentBeginOverlap`
  (params (OverlappedComponent :type "PrimitiveComponent Object Reference") (OtherActor :type "Actor Object Reference") (OtherComp :type "PrimitiveComponent Object Reference") (OtherBodyIndex :type Integer) (bFromSweep :type Boolean) (SweepResult :type "HitResult Structure (by ref)"))
  (bind _shieldgrowth (`self.ShieldGrowth`))
  (if (`KismetSystemLibrary.K2_IsValidTimerHandle` _shieldgrowth)
    (`KismetSystemLibrary.K2_ClearAndInvalidateTimerHandle` _shieldgrowth))
  (cast `ShooterSandboxCharacter` OtherActor)
  (bind _returnvalue (`KismetSystemLibrary.K2_SetTimerDelegate` (delegate `ShieldShrink`) 0.05 true))
  (set `self.ShieldGrowth` _returnvalue)
  (`/Engine/EditorBlueprintResources/StandardMacros.IncrementInt` (`self.NumPlayerInVicinity`)))

(event `ShieldShrink`
  (bind _towershield (`self.TowerShield`))
  (bind (_returnvalue_x _returnvalue_y _returnvalue_z) (`KismetMathLibrary.BreakVector` (`SceneComponent.K2_GetComponentScale` _towershield)))
  (`SceneComponent.SetWorldScale3D` _towershield (`KismetMathLibrary.MakeVector` _returnvalue_x (`KismetMathLibrary.FInterpTo` _returnvalue_y (`self.ShieldShrunkHeight`) 0.05 2.0) _returnvalue_z))
  (if (`KismetMathLibrary.NearlyEqual_FloatFloat` (.y (`SceneComponent.K2_GetComponentScale` _towershield)) (`self.ShieldShrunkHeight`) 0.1)
    (`KismetSystemLibrary.K2_ClearAndInvalidateTimerHandle` (`self.ShieldGrowth`))))

(event `self.Vicinity.OnComponentEndOverlap`
  (params (OverlappedComponent :type "PrimitiveComponent Object Reference") (OtherActor :type "Actor Object Reference") (OtherComp :type "PrimitiveComponent Object Reference") (OtherBodyIndex :type Integer))
  (bind _shieldgrowth (`self.ShieldGrowth`))
  (if (`KismetSystemLibrary.K2_IsValidTimerHandle` _shieldgrowth)
    (`KismetSystemLibrary.K2_ClearAndInvalidateTimerHandle` _shieldgrowth))
  (cast `ShooterSandboxCharacter` OtherActor)
  (bind _result (`/Engine/EditorBlueprintResources/StandardMacros.DecrementInt` (`self.NumPlayerInVicinity`))
    (:`  `
      (if (< _result 1)
        (bind _returnvalue (`KismetSystemLibrary.K2_SetTimerDelegate` (delegate `ShieldExpand`) 0.05 true))
        (set `self.ShieldGrowth` _returnvalue)))))

(event `ShieldExpand`
  (bind _towershield (`self.TowerShield`))
  (bind (_returnvalue_x _returnvalue_y _returnvalue_z) (`KismetMathLibrary.BreakVector` (`SceneComponent.K2_GetComponentScale` _towershield)))
  (`SceneComponent.SetWorldScale3D` _towershield (`KismetMathLibrary.MakeVector` _returnvalue_x (`KismetMathLibrary.FInterpTo` _returnvalue_y (`self.ShieldOriginalHeight`) 0.05 2.0) _returnvalue_z))
  (if (`KismetMathLibrary.NearlyEqual_FloatFloat` (.y (`SceneComponent.K2_GetComponentScale` _towershield)) (`self.ShieldOriginalHeight`) 0.1)
    (`KismetSystemLibrary.K2_ClearAndInvalidateTimerHandle` (`self.ShieldGrowth`))))

(event `self.LiftPad.OnComponentBeginOverlap`
  (params (OverlappedComponent :type "PrimitiveComponent Object Reference") (OtherActor :type "Actor Object Reference") (OtherComp :type "PrimitiveComponent Object Reference") (OtherBodyIndex :type Integer) (bFromSweep :type Boolean) (SweepResult :type "HitResult Structure (by ref)"))
  (cast `ShooterSandboxCharacter` OtherActor)
  (bind (_direction _liftposition) (`Timeline|LiftUp` :!label _label)
    (:`Update`
      (`SceneComponent.K2_SetRelativeLocation` (`self.TowerLift`) (`KismetMathLibrary.VLerp` (`self.LiftDownPosition`) (`self.LiftUpPosition`) _liftposition) false false))))

(event `self.LiftPad.OnComponentEndOverlap`
  (params (OverlappedComponent :type "PrimitiveComponent Object Reference") (OtherActor :type "Actor Object Reference") (OtherComp :type "PrimitiveComponent Object Reference") (OtherBodyIndex :type Integer))
  (cast `ShooterSandboxCharacter` OtherActor)
  (`KismetSystemLibrary.PrintString` "Overlap ended")
  (goto _label :!via `Reverse`))

(event `self.PlatformTrigerFwd.OnComponentBeginOverlap`
  (params (OverlappedComponent :type "PrimitiveComponent Object Reference") (OtherActor :type "Actor Object Reference") (OtherComp :type "PrimitiveComponent Object Reference") (OtherBodyIndex :type Integer) (bFromSweep :type Boolean) (SweepResult :type "HitResult Structure (by ref)"))
  (`/Engine/EditorBlueprintResources/ActorMacros.Switch Has Authority`
    (:`Authority`
      (cast `ShooterSandboxCharacter` OtherActor)
      (`self.SpawnPlatformAt` (`self.PlatformTrigerFwd`)))))

(event `self.PlatformTrigerBwd.OnComponentBeginOverlap`
  (params (OverlappedComponent :type "PrimitiveComponent Object Reference") (OtherActor :type "Actor Object Reference") (OtherComp :type "PrimitiveComponent Object Reference") (OtherBodyIndex :type Integer) (bFromSweep :type Boolean) (SweepResult :type "HitResult Structure (by ref)"))
  (`/Engine/EditorBlueprintResources/ActorMacros.Switch Has Authority`
    (:`Authority`
      (cast `ShooterSandboxCharacter` OtherActor)
      (`self.SpawnPlatformAt` (`self.PlatformTrigerBwd`)))))

(event `self.PlatformTrigerRight.OnComponentBeginOverlap`
  (params (OverlappedComponent :type "PrimitiveComponent Object Reference") (OtherActor :type "Actor Object Reference") (OtherComp :type "PrimitiveComponent Object Reference") (OtherBodyIndex :type Integer) (bFromSweep :type Boolean) (SweepResult :type "HitResult Structure (by ref)"))
  (`/Engine/EditorBlueprintResources/ActorMacros.Switch Has Authority`
    (:`Authority`
      (cast `ShooterSandboxCharacter` OtherActor)
      (`self.SpawnPlatformAt` (`self.PlatformTrigerRight`)))))

(event `self.PlatformTrigerLeft.OnComponentBeginOverlap`
  (params (OverlappedComponent :type "PrimitiveComponent Object Reference") (OtherActor :type "Actor Object Reference") (OtherComp :type "PrimitiveComponent Object Reference") (OtherBodyIndex :type Integer) (bFromSweep :type Boolean) (SweepResult :type "HitResult Structure (by ref)"))
  (`/Engine/EditorBlueprintResources/ActorMacros.Switch Has Authority`
    (:`Authority`
      (cast `ShooterSandboxCharacter` OtherActor)
      (`self.SpawnPlatformAt` (`self.PlatformTrigerLeft`)))))

(event `SpawnPlatformAt`
  (params (TriggeredPad :type "StaticMeshComponent Object Reference"))
  (bind _returnvalue (`|SpawnActorFromClass` "/Game/Blueprints/Constructs/ChainPlatform.ChainPlatform_C" (`KismetMathLibrary.MakeTransform` (+ (`SceneComponent.K2_GetComponentLocation` TriggeredPad) (* (`SceneComponent.GetForwardVector` TriggeredPad) 1000)) (`SceneComponent.K2_GetComponentRotation` TriggeredPad)) "AdjustIfPossibleButDontSpawnIfColliding" "OverrideRootScale" null null))
  (`/Engine/EditorBlueprintResources/StandardMacros.IsValid` _returnvalue))

(fn `UserConstructionScript`)