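; ChainPlatform is a platform actor that extends itself by spawning further copies when a ShooterSandboxCharacter touches one of its forward, right or left triggers.
; Each overlap runs only with authority and passes the trigger to SpawnPlatformAt, which places a new platform a fixed distance along that trigger's forward vector, matching its rotation.
; Collision handling adjusts placement or cancels blocked spawns, and a debug print reports the result.
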(event `self.PlatformTrigerFwd.OnComponentBeginOverlap`
  (params (OverlappedComponent :type "PrimitiveComponent Object Reference") (OtherActor :type "Actor Object Reference") (OtherComp :type "PrimitiveComponent Object Reference") (OtherBodyIndex :type Integer) (bFromSweep :type Boolean) (SweepResult :type "HitResult Structure (by ref)"))
  (`/Engine/EditorBlueprintResources/ActorMacros.Switch Has Authority`
    (:`Authority`
      (cast `ShooterSandboxCharacter` OtherActor)
      (`self.SpawnPlatformAt` (`self.PlatformTrigerFwd`)))))

(event `self.PlatformTrigerRight.OnComponentBeginOverlap`
  (params (OverlappedComponent :type "PrimitiveComponent Object Reference") (OtherActor :type "Actor Object Reference") (OtherComp :type "PrimitiveComponent Object Reference") (OtherBodyIndex :type Integer) (bFromSweep :type Boolean) (SweepResult :type "HitResult Structure (by ref)"))
  (`/Engine/EditorBlueprintResources/ActorMacros.Switch Has Authority`
    (:`Authority`
      (cast `ShooterSandboxCharacter` OtherActor)
      (`self.SpawnPlatformAt` (`self.PlatformTrigerRight`)))))

(event `self.PlatformTrigerLeft.OnComponentBeginOverlap`
  (params (OverlappedComponent :type "PrimitiveComponent Object Reference") (OtherActor :type "Actor Object Reference") (OtherComp :type "PrimitiveComponent Object Reference") (OtherBodyIndex :type Integer) (bFromSweep :type Boolean) (SweepResult :type "HitResult Structure (by ref)"))
  (`/Engine/EditorBlueprintResources/ActorMacros.Switch Has Authority`
    (:`Authority`
      (cast `ShooterSandboxCharacter` OtherActor)
      (`self.SpawnPlatformAt` (`self.PlatformTrigerLeft`)))))

(event `SpawnPlatformAt`
  (params (TriggeredPad :type "StaticMeshComponent Object Reference"))
  (bind _returnvalue (`|SpawnActorFromClass` "ChainPlatform_C" (`KismetMathLibrary.MakeTransform` (+ (`SceneComponent.K2_GetComponentLocation` TriggeredPad) (* (`SceneComponent.GetForwardVector` TriggeredPad) 1000)) (`SceneComponent.K2_GetComponentRotation` TriggeredPad)) "AdjustIfPossibleButDontSpawnIfColliding" "OverrideRootScale" null null))
  (`/Engine/EditorBlueprintResources/StandardMacros.IsValid` _returnvalue
    (:`Is Valid`
      (`KismetSystemLibrary.PrintString` "spawned"))
    (:`Is Not Valid`
      (`KismetSystemLibrary.PrintString` "NOT spawned"))))

(fn `UserConstructionScript`)