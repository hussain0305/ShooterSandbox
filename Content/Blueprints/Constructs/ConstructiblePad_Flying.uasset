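; Flying constructible pad with four spinning rotors that wanders on world axes, avoiding obstacles.
; After a startup delay, the server starts a self-repeating probe loop of six sphere traces, while Tick moves it along the current direction.
; When that direction is blocked, it picks randomly among clear ones, though Left is always a candidate, even if blocked.
; A self-restarting timeline spins the rotors.
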(event `self.ReceiveTick`
  (params (DeltaSeconds :type "Float (single-precision)"))
  (if (`self.CanFly`)
    (`/Engine/EditorBlueprintResources/ActorMacros.Switch Has Authority`
      (:`Authority`
        (switch `/Game/Data/Enum_NavDirections` (`self.CurrentDirection`)
          (:`NewEnumerator0`
            (`self.AddMovementInput` self (0.0 0.0 5.0) 1.0 false))
          (:`NewEnumerator1`
            (`self.AddMovementInput` self (0.0 0.0 -5.0) 1.0 false))
          (:`NewEnumerator2`
            (`self.AddMovementInput` self (5.0 0.0 0.0) 1.0 false))
          (:`NewEnumerator3`
            (`self.AddMovementInput` self (-5.0 0.0 0.0) 1.0 false))
          (:`NewEnumerator4`
            (`self.AddMovementInput` self (0.0 5.0 0.0) 1.0 false))
          (:`NewEnumerator5`
            (`self.AddMovementInput` self (0.0 -5.0 0.0) 1.0 false)))))))

(event `GoInDirection`
  (params (Direction :type "/Game/Data/Enum_NavDirections Enum" :default "NewEnumerator0"))
  (set `self.CurrentDirection` Direction))

(event `self.ReceiveBeginPlay`
  (`self.RotateRotor`)
  (`self.PrepProbeIgnore`)
  (`/Engine/EditorBlueprintResources/ActorMacros.Switch Has Authority`
    (:`Authority`
      (`KismetSystemLibrary.Delay` 10.0)
      (set `self.CanFly` true)
      (`self.StartNavigating`)
      (`self.GoInDirection` "NewEnumerator2"))))

(event `PrepProbeIgnore`
  (set `self.ProbeIgnore` (`|MakeArray` self :!type "Actor Object Reference")))

(event `RotateRotor`
  (bind (_direction _rotation) (`Timeline|RotorRotation` :!via `PlayFromStart`)
    (:`Update`
      (`/Engine/EditorBlueprintResources/StandardMacros.IsValid` (`self.Rotor_1`)
        (:`Is Valid`
          (`SceneComponent.K2_SetRelativeRotation` (`self.Rotor_1`) (`KismetMathLibrary.MakeRotator` 0.0 0.0 _rotation) false false))
        (:`Is Not Valid`
          _))
      (`/Engine/EditorBlueprintResources/StandardMacros.IsValid` (`self.Rotor_2`)
        (:`Is Valid`
          (`SceneComponent.K2_SetRelativeRotation` (`self.Rotor_2`) (`KismetMathLibrary.MakeRotator` 0.0 0.0 _rotation) false false))
        (:`Is Not Valid`
          _))
      (`/Engine/EditorBlueprintResources/StandardMacros.IsValid` (`self.Rotor_3`)
        (:`Is Valid`
          (`SceneComponent.K2_SetRelativeRotation` (`self.Rotor_3`) (`KismetMathLibrary.MakeRotator` 0.0 0.0 _rotation) false false))
        (:`Is Not Valid`
          _))
      (`/Engine/EditorBlueprintResources/StandardMacros.IsValid` (`self.Rotor_4`)
        (:`Is Valid`
          (`SceneComponent.K2_SetRelativeRotation` (`self.Rotor_4`) (`KismetMathLibrary.MakeRotator` 0.0 0.0 _rotation) false false))))
    (:`Finished`
      (`self.RotateRotor`))))

(event `StartNavigating`
  (bind _returnvalue (`self.K2_GetActorLocation`))
  (bind _returnvalue_2 (`self.K2_GetActorLocation`))
  (bind _returnvalue_3 (`self.K2_GetActorLocation`))
  (bind _returnvalue_4 (`self.K2_GetActorLocation`))
  (bind _returnvalue_5 (`self.K2_GetActorLocation`))
  (bind _returnvalue_6 (`self.K2_GetActorLocation`))
  (bind (_proberesults_up _proberesults_down _proberesults_forward _proberesults_backward _proberesults_right _proberesults_left) (break `/Game/Data/NavigationDirections` (`self.ProbeResults`)))
  (bind (_proberesults_up_2 _proberesults_down_2 _proberesults_forward_2 _proberesults_backward_2 _proberesults_right_2 _proberesults_left_2) (break `/Game/Data/NavigationDirections` (`self.ProbeResults`)))
  (bind (_proberesults_up_3 _proberesults_down_3 _proberesults_forward_3 _proberesults_backward_3 _proberesults_right_3) (break `/Game/Data/NavigationDirections` (`self.ProbeResults`)))
  (bind (_proberesults_up_4 _proberesults_down_4 _proberesults_forward_4 _proberesults_backward_4 _proberesults_right_4 _proberesults_left_3) (break `/Game/Data/NavigationDirections` (`self.ProbeResults`)))
  (bind (_proberesults_up_5 _proberesults_down_5 _proberesults_forward_5 _proberesults_backward_5 _proberesults_right_5 _proberesults_left_4) (break `/Game/Data/NavigationDirections` (`self.ProbeResults`)))
  (bind (_proberesults_up_6 _proberesults_down_6 _proberesults_forward_6 _proberesults_backward_6 _proberesults_right_6 _proberesults_left_5) (break `/Game/Data/NavigationDirections` (`self.ProbeResults`)))
  (bind (_outhit _returnvalue_7) (`KismetSystemLibrary.SphereTraceSingle` (+ _returnvalue_3 (-1500.0 2000.0 1200.0)) (+ _returnvalue_3 (1500.0 2000.0 1200.0)) (`self.TraceSize`) "TraceTypeQuery1" false (`self.ProbeIgnore`) "None" true (struct :`R` 1.0 :`A` 1.0) (struct :`G` 1.0 :`A` 1.0) 0.1))
  (set `self.ProbeResults` (make `/Game/Data/NavigationDirections` _proberesults_up_6 _proberesults_down_6 _proberesults_forward_6 _proberesults_backward_6 _returnvalue_7 _proberesults_left_5))
  (bind (_outhit_2 _returnvalue_8) (`KismetSystemLibrary.SphereTraceSingle` (+ _returnvalue_4 (-1500.0 -2000.0 1200.0)) (+ _returnvalue_4 (1500.0 -2000.0 1200.0)) (`self.TraceSize`) "TraceTypeQuery1" false (`self.ProbeIgnore`) "None" true (struct :`R` 1.0 :`A` 1.0) (struct :`G` 1.0 :`A` 1.0) 0.1))
  (set `self.ProbeResults` (make `/Game/Data/NavigationDirections` _proberesults_up_3 _proberesults_down_3 _proberesults_forward_3 _proberesults_backward_3 _proberesults_right_3 _returnvalue_8))
  (bind (_outhit_3 _returnvalue_9) (`KismetSystemLibrary.SphereTraceSingle` (+ _returnvalue_5 (-2000.0 -1500.0 1200.0)) (+ _returnvalue_5 (-2000.0 1500.0 1200.0)) (`self.TraceSize`) "TraceTypeQuery1" false (`self.ProbeIgnore`) "None" true (struct :`R` 1.0 :`A` 1.0) (struct :`G` 1.0 :`A` 1.0) 0.1))
  (set `self.ProbeResults` (make `/Game/Data/NavigationDirections` _proberesults_up _proberesults_down _proberesults_forward _returnvalue_9 _proberesults_right _proberesults_left))
  (bind (_outhit_4 _returnvalue_10) (`KismetSystemLibrary.SphereTraceSingle` (+ _returnvalue_6 (2000.0 -1500.0 1200.0)) (+ _returnvalue_6 (2000.0 1500.0 1200.0)) (`self.TraceSize`) "TraceTypeQuery1" false (`self.ProbeIgnore`) "None" true (struct :`R` 1.0 :`A` 1.0) (struct :`G` 1.0 :`A` 1.0) 0.1))
  (set `self.ProbeResults` (make `/Game/Data/NavigationDirections` _proberesults_up_4 _proberesults_down_4 _returnvalue_10 _proberesults_backward_4 _proberesults_right_4 _proberesults_left_3))
  (bind (_outhit_5 _returnvalue_11) (`KismetSystemLibrary.SphereTraceSingle` (+ _returnvalue_2 (0.0 0.0 1800.0)) (+ _returnvalue_2 (0.0 0.0 2800.0)) (`self.TraceSizeVertical`) "TraceTypeQuery1" false (`self.ProbeIgnore`) "None" true (struct :`R` 1.0 :`A` 1.0) (struct :`G` 1.0 :`A` 1.0) 0.1))
  (set `self.ProbeResults` (make `/Game/Data/NavigationDirections` _returnvalue_11 _proberesults_down_2 _proberesults_forward_2 _proberesults_backward_2 _proberesults_right_2 _proberesults_left_2))
  (bind (_outhit_6 _returnvalue_12) (`KismetSystemLibrary.SphereTraceSingle` (+ _returnvalue (0.0 0.0 -600.0)) (+ _returnvalue (0.0 0.0 400.0)) (`self.TraceSizeVertical`) "TraceTypeQuery1" false (`self.ProbeIgnore`) "None" true (struct :`R` 1.0 :`A` 1.0) (struct :`G` 1.0 :`A` 1.0) 0.1))
  (set `self.ProbeResults` (make `/Game/Data/NavigationDirections` _proberesults_up_5 _returnvalue_12 _proberesults_forward_5 _proberesults_backward_5 _proberesults_right_5 _proberesults_left_4))
  (`self.EvaluatePath`)
  (`KismetSystemLibrary.Delay` 0.2)
  (`self.StartNavigating`))

(event `EvaluatePath`
  (bind (_proberesults_up _proberesults_down _proberesults_forward _proberesults_backward _proberesults_right _proberesults_left) (break `/Game/Data/NavigationDirections` (`self.ProbeResults`)))
  (switch `/Game/Data/Enum_NavDirections` (`self.CurrentDirection`)
    (:`NewEnumerator0`
      (if _proberesults_up
        (`self.DecideWhereToGo` :!label _label)))
    (:`NewEnumerator1`
      (if _proberesults_down
        (goto _label)))
    (:`NewEnumerator2`
      (if _proberesults_forward
        (goto _label)))
    (:`NewEnumerator3`
      (if _proberesults_backward
        (goto _label)))
    (:`NewEnumerator4`
      (if _proberesults_right
        (goto _label)))
    (:`NewEnumerator5`
      (if _proberesults_left
        (goto _label)))))

(event `DecideWhereToGo`
  (bind _availabledirectionstogo (`self.AvailableDirectionsToGo`))
  (bind (_proberesults_up _proberesults_down _proberesults_forward _proberesults_backward _proberesults_right _proberesults_left) (break `/Game/Data/NavigationDirections` (`self.ProbeResults`)))
  (set `self.AvailableDirectionsToGo` (`|MakeArray`))
  (if (not _proberesults_up)
    (`KismetArrayLibrary.Array_Add` (`self.AvailableDirectionsToGo`) "NewEnumerator0"))
  (if (not _proberesults_down)
    (`KismetArrayLibrary.Array_Add` (`self.AvailableDirectionsToGo`) "NewEnumerator1"))
  (if (not _proberesults_forward)
    (`KismetArrayLibrary.Array_Add` (`self.AvailableDirectionsToGo`) "NewEnumerator2"))
  (if (not _proberesults_backward)
    (`KismetArrayLibrary.Array_Add` (`self.AvailableDirectionsToGo`) "NewEnumerator3"))
  (if (not _proberesults_right)
    (`KismetArrayLibrary.Array_Add` (`self.AvailableDirectionsToGo`) "NewEnumerator4"))
  (if (not _proberesults_left)
    _
    (else
      _))
  (`KismetArrayLibrary.Array_Add` (`self.AvailableDirectionsToGo`) "NewEnumerator5")
  (`self.GoInDirection` (`|GetArrayItem` _availabledirectionstogo (`KismetMathLibrary.RandomInteger` (`KismetArrayLibrary.Array_Length` _availabledirectionstogo)))))

(fn `UserConstructionScript`)