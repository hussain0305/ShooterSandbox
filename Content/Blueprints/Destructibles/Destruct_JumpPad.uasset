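; Destructible jump pad actor that breaks apart when ConstructDestruction is called with a material and a low, mid or high variant.
; It destroys the two unused destructible components and applies the given material to several slots of the remaining one.
; It then shatters that mesh with full radial damage at the actor's location, using a random radius and an impulse that grows from low to high.
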(event `self.ConstructDestruction`
  (params (materialToApply :type "MaterialInstance Object Reference") (lowMidHigh :type Integer))
  (bind _destructiblehigh (`self.DestructibleHigh`))
  (bind _destructiblelow (`self.DestructibleLow`))
  (bind _destructiblemid (`self.DestructibleMid`))
  (switch `int` lowMidHigh
    (:`1`
      (`ActorComponent.K2_DestroyComponent` (`self.DestructibleMid`))
      (`ActorComponent.K2_DestroyComponent` (`self.DestructibleHigh`))
      (`PrimitiveComponent.SetMaterial` _destructiblelow 0 materialToApply)
      (`PrimitiveComponent.SetMaterial` _destructiblelow 1 materialToApply)
      (`PrimitiveComponent.SetMaterial` _destructiblelow 3 materialToApply)
      (`DestructibleComponent.ApplyRadiusDamage` _destructiblelow 1000.0 (`self.K2_GetActorLocation`) (`KismetMathLibrary.RandomFloatInRange` 100.0 250.0) 25000.0 true))
    (:`2`
      (`ActorComponent.K2_DestroyComponent` (`self.DestructibleLow`))
      (`ActorComponent.K2_DestroyComponent` (`self.DestructibleHigh`))
      (`PrimitiveComponent.SetMaterial` _destructiblemid 0 materialToApply)
      (`PrimitiveComponent.SetMaterial` _destructiblemid 1 materialToApply)
      (`PrimitiveComponent.SetMaterial` _destructiblemid 3 materialToApply)
      (`DestructibleComponent.ApplyRadiusDamage` _destructiblemid 1000.0 (`self.K2_GetActorLocation`) (`KismetMathLibrary.RandomFloatInRange` 100.0 250.0) 30000.0 true))
    (:`3`
      (`ActorComponent.K2_DestroyComponent` (`self.DestructibleMid`))
      (`ActorComponent.K2_DestroyComponent` (`self.DestructibleLow`))
      (`PrimitiveComponent.SetMaterial` _destructiblehigh 0 materialToApply)
      (`PrimitiveComponent.SetMaterial` _destructiblehigh 1 materialToApply)
      (`PrimitiveComponent.SetMaterial` _destructiblehigh 3 materialToApply)
      (`DestructibleComponent.ApplyRadiusDamage` _destructiblehigh 1000.0 (`self.K2_GetActorLocation`) (`KismetMathLibrary.RandomFloatInRange` 100.0 250.0) 45000.0 true))))

(fn `UserConstructionScript`)