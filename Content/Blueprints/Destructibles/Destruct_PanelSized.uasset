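; Panel-sized destructible actor that takes on a supplied material and scale, then shatters on command.
; ConstructDestruction debug-prints the material name, assigns it to three of the Destructible component's slots, and sets world scale to the given scale divided by a scale factor.
; It then applies full radius damage at the actor's location, using the passed force as both damage and impulse to break the mesh.
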(event `self.ConstructDestruction`
  (params (scale :type "Vector Structure") (materialToApply :type "MaterialInstance Object Reference") (forceVal :type "Float (single-precision)") (scaleFactor :type "Float (single-precision)"))
  (bind _destructible (`self.Destructible`))
  (`KismetSystemLibrary.PrintString` (`KismetSystemLibrary.GetDisplayName` materialToApply))
  (`PrimitiveComponent.SetMaterial` _destructible 0 materialToApply)
  (`PrimitiveComponent.SetMaterial` _destructible 1 materialToApply)
  (`PrimitiveComponent.SetMaterial` _destructible 3 materialToApply)
  (`SceneComponent.SetWorldScale3D` _destructible (/ scale scaleFactor))
  (`DestructibleComponent.ApplyRadiusDamage` _destructible forceVal (`self.K2_GetActorLocation`) 600.0 forceVal true))

(fn `UserConstructionScript`)