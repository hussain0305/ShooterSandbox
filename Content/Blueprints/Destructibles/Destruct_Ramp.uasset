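; Destructible ramp actor that shatters as soon as its ConstructDestruction event is called with a material and a low, mid or high level.
; It keeps the matching one of three destructible components, destroys the other two and applies the passed material to several of its slots.
; It then fractures that component with full radius damage from a randomized point above the actor, using a stronger impulse at higher levels.
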(event `self.ConstructDestruction`
  (params (materialToApply :type "MaterialInstance Object Reference") (lowMidHigh :type Integer))
  (bind _destructiblehigh (`self.DestructibleHigh`))
  (bind _destructiblelow (`self.DestructibleLow`))
  (bind _destructiblemid (`self.DestructibleMid`))
  (switch `int` lowMidHigh
    (:`1`
      (`ActorComponent.K2_DestroyComponent` (`self.DestructibleMid`))
      (`ActorComponent.K2_DestroyComponent` (`self.DestructibleHigh`))
      (`PrimitiveComponent.SetMaterial` _destructiblelow 0 materialToApply)
      (`PrimitiveComponent.SetMaterial` _destructiblelow 1 materialToApply)
      (`PrimitiveComponent.SetMaterial` _destructiblelow 3 materialToApply)
      (`DestructibleComponent.ApplyRadiusDamage` _destructiblelow 5000.0 (`KismetMathLibrary.MakeVector` (.x (`self.K2_GetActorLocation`)) (.y (`self.K2_GetActorLocation`)) (+ (.z (`self.K2_GetActorLocation`)) (`KismetMathLibrary.RandomFloatInRange` 150.0 300.0))) (`KismetMathLibrary.RandomFloatInRange` 100.0 250.0) 25000.0 true))
    (:`2`
      (`ActorComponent.K2_DestroyComponent` (`self.DestructibleLow`))
      (`ActorComponent.K2_DestroyComponent` (`self.DestructibleHigh`))
      (`PrimitiveComponent.SetMaterial` _destructiblemid 0 materialToApply)
      (`PrimitiveComponent.SetMaterial` _destructiblemid 1 materialToApply)
      (`PrimitiveComponent.SetMaterial` _destructiblemid 3 materialToApply)
      (`DestructibleComponent.ApplyRadiusDamage` _destructiblemid 5000.0 (`KismetMathLibrary.MakeVector` (.x (`self.K2_GetActorLocation`)) (.y (`self.K2_GetActorLocation`)) (+ (.z (`self.K2_GetActorLocation`)) (`KismetMathLibrary.RandomFloatInRange` 150.0 300.0))) (`KismetMathLibrary.RandomFloatInRange` 100.0 250.0) 75000.0 true))
    (:`3`
      (`ActorComponent.K2_DestroyComponent` (`self.DestructibleMid`))
      (`ActorComponent.K2_DestroyComponent` (`self.DestructibleLow`))
      (`PrimitiveComponent.SetMaterial` _destructiblehigh 0 materialToApply)
      (`PrimitiveComponent.SetMaterial` _destructiblehigh 1 materialToApply)
      (`PrimitiveComponent.SetMaterial` _destructiblehigh 3 materialToApply)
      (`DestructibleComponent.ApplyRadiusDamage` _destructiblehigh 5000.0 (`KismetMathLibrary.MakeVector` (.x (`self.K2_GetActorLocation`)) (.y (`self.K2_GetActorLocation`)) (+ (.z (`self.K2_GetActorLocation`)) (`KismetMathLibrary.RandomFloatInRange` 150.0 300.0))) (`KismetMathLibrary.RandomFloatInRange` 100.0 250.0) 100000.0 true))))

(fn `UserConstructionScript`)