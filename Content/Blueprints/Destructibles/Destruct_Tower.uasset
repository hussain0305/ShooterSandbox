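; Destructible tower that breaks apart in one of three Low, Mid or High variants, each made of body, shield and platform pieces.
; ConstructDestruction keeps the pieces for the chosen variant and destroys the others.
; It teleports the kept pieces upward, applies tower materials and fractures them with full radius damage.
; Impulse strength rises from Low to High, and body damage originates at the shield's location.
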(event `self.ConstructDestruction`
  (params (materialToApply :type "MaterialInstance Object Reference") (lowMidHigh :type Integer))
  (bind _towerbodyhigh (`self.TowerBodyHigh`))
  (bind _shieldhigh (`self.ShieldHigh`))
  (bind _platformhigh (`self.PlatformHigh`))
  (bind _towerbodylow (`self.TowerBodyLow`))
  (bind _shieldlow (`self.ShieldLow`))
  (bind _platformlow (`self.PlatformLow`))
  (bind _towerbodymid (`self.TowerBodyMid`))
  (bind _shieldmid (`self.ShieldMid`))
  (bind _platformmid (`self.PlatformMid`))
  (bind _returnvalue (`SceneComponent.K2_GetComponentLocation` _shieldmid))
  (bind _returnvalue_2 (`SceneComponent.K2_GetComponentLocation` _shieldlow))
  (bind _returnvalue_3 (`SceneComponent.K2_GetComponentLocation` _shieldhigh))
  (switch `int` lowMidHigh
    (:`1`
      (`ActorComponent.K2_DestroyComponent` (`self.TowerBodyMid`))
      (`ActorComponent.K2_DestroyComponent` (`self.TowerBodyHigh`))
      (`ActorComponent.K2_DestroyComponent` (`self.ShieldMid`))
      (`ActorComponent.K2_DestroyComponent` (`self.PlatformHigh`))
      (`ActorComponent.K2_DestroyComponent` (`self.PlatformMid`))
      (`ActorComponent.K2_DestroyComponent` (`self.ShieldHigh`))
      (`SceneComponent.K2_AddLocalOffset` _towerbodylow (0.0 0.0 1500.0) false true)
      (`PrimitiveComponent.SetMaterial` _towerbodylow 0 "/Game/Materials/Glow/Tower/Tower1.Tower1")
      (`PrimitiveComponent.SetMaterial` _towerbodylow 1 "/Game/Materials/Glow/Tower/Tower1.Tower1")
      (`PrimitiveComponent.SetMaterial` _towerbodylow 3 "/Game/Materials/Glow/Tower/Tower1.Tower1")
      (`DestructibleComponent.ApplyRadiusDamage` _towerbodylow 1000.0 _returnvalue_2 3000.0 50000.0 true)
      (`SceneComponent.K2_AddLocalOffset` _shieldlow (0.0 0.0 1500.0) false true)
      (`PrimitiveComponent.SetMaterial` _shieldlow 0 "/Game/Materials/Glow/Tower/Tower.Tower")
      (`PrimitiveComponent.SetMaterial` _shieldlow 1 "/Game/Materials/Glow/Tower/Tower.Tower")
      (`PrimitiveComponent.SetMaterial` _shieldlow 3 "/Game/Materials/Glow/Tower/Tower.Tower")
      (`DestructibleComponent.ApplyRadiusDamage` _shieldlow 1000.0 _returnvalue_2 3000.0 50000.0 true)
      (`SceneComponent.K2_AddLocalOffset` _platformlow (0.0 0.0 3000.0) false true)
      (`PrimitiveComponent.SetMaterial` _platformlow 0 "/Game/Materials/Glow/Tower/Tower2.Tower2")
      (`PrimitiveComponent.SetMaterial` _platformlow 1 "/Game/Materials/Glow/Tower/Tower2.Tower2")
      (`PrimitiveComponent.SetMaterial` _platformlow 3 "/Game/Materials/Glow/Tower/Tower2.Tower2")
      (`DestructibleComponent.ApplyRadiusDamage` _platformlow 1000.0 (`SceneComponent.K2_GetComponentLocation` _platformlow) 500.0 25000.0 true))
    (:`2`
      (`ActorComponent.K2_DestroyComponent` (`self.TowerBodyLow`))
      (`ActorComponent.K2_DestroyComponent` (`self.TowerBodyHigh`))
      (`ActorComponent.K2_DestroyComponent` (`self.ShieldLow`))
      (`ActorComponent.K2_DestroyComponent` (`self.PlatformHigh`))
      (`ActorComponent.K2_DestroyComponent` (`self.PlatformLow`))
      (`ActorComponent.K2_DestroyComponent` (`self.ShieldHigh`))
      (`SceneComponent.K2_AddLocalOffset` _towerbodymid (0.0 0.0 1500.0) false true)
      (`PrimitiveComponent.SetMaterial` _towerbodymid 0 "/Game/Materials/Glow/Tower/Tower1.Tower1")
      (`PrimitiveComponent.SetMaterial` _towerbodymid 1 "/Game/Materials/Glow/Tower/Tower1.Tower1")
      (`PrimitiveComponent.SetMaterial` _towerbodymid 3 "/Game/Materials/Glow/Tower/Tower1.Tower1")
      (`DestructibleComponent.ApplyRadiusDamage` _towerbodymid 1000.0 _returnvalue 3000.0 100000.0 true)
      (`SceneComponent.K2_AddLocalOffset` _shieldmid (0.0 0.0 1500.0) false true)
      (`PrimitiveComponent.SetMaterial` _shieldmid 0 "/Game/Materials/Glow/Tower/Tower.Tower")
      (`PrimitiveComponent.SetMaterial` _shieldmid 1 "/Game/Materials/Glow/Tower/Tower.Tower")
      (`PrimitiveComponent.SetMaterial` _shieldmid 3 "/Game/Materials/Glow/Tower/Tower.Tower")
      (`DestructibleComponent.ApplyRadiusDamage` _shieldmid 1000.0 _returnvalue 3000.0 100000.0 true)
      (`SceneComponent.K2_AddLocalOffset` _platformmid (0.0 0.0 3000.0) false true)
      (`PrimitiveComponent.SetMaterial` _platformmid 0 "/Game/Materials/Glow/Tower/Tower2.Tower2")
      (`PrimitiveComponent.SetMaterial` _platformmid 1 "/Game/Materials/Glow/Tower/Tower2.Tower2")
      (`PrimitiveComponent.SetMaterial` _platformmid 3 "/Game/Materials/Glow/Tower/Tower2.Tower2")
      (`DestructibleComponent.ApplyRadiusDamage` _platformmid 1000.0 (`SceneComponent.K2_GetComponentLocation` _platformmid) 500.0 50000.0 true))
    (:`3`
      (`ActorComponent.K2_DestroyComponent` (`self.TowerBodyMid`))
      (`ActorComponent.K2_DestroyComponent` (`self.ShieldLow`))
      (`ActorComponent.K2_DestroyComponent` (`self.ShieldMid`))
      (`ActorComponent.K2_DestroyComponent` (`self.PlatformLow`))
      (`ActorComponent.K2_DestroyComponent` (`self.PlatformMid`))
      (`ActorComponent.K2_DestroyComponent` (`self.TowerBodyLow`))
      (`SceneComponent.K2_AddLocalOffset` _towerbodyhigh (0.0 0.0 1500.0) false true)
      (`PrimitiveComponent.SetMaterial` _towerbodyhigh 0 "/Game/Materials/Glow/Tower/Tower1.Tower1")
      (`PrimitiveComponent.SetMaterial` _towerbodyhigh 1 "/Game/Materials/Glow/Tower/Tower1.Tower1")
      (`PrimitiveComponent.SetMaterial` _towerbodyhigh 3 "/Game/Materials/Glow/Tower/Tower1.Tower1")
      (`DestructibleComponent.ApplyRadiusDamage` _towerbodyhigh 1000.0 _returnvalue_3 3000.0 150000.0 true)
      (`SceneComponent.K2_AddLocalOffset` _shieldhigh (0.0 0.0 1500.0) false true)
      (`PrimitiveComponent.SetMaterial` _shieldhigh 0 "/Game/Materials/Glow/Tower/Tower.Tower")
      (`PrimitiveComponent.SetMaterial` _shieldhigh 1 "/Game/Materials/Glow/Tower/Tower.Tower")
      (`PrimitiveComponent.SetMaterial` _shieldhigh 3 "/Game/Materials/Glow/Tower/Tower.Tower")
      (`DestructibleComponent.ApplyRadiusDamage` _shieldhigh 1000.0 _returnvalue_3 3000.0 150000.0 true)
      (`SceneComponent.K2_AddLocalOffset` _platformhigh (0.0 0.0 3000.0) false true)
      (`PrimitiveComponent.SetMaterial` _platformhigh 0 "/Game/Materials/Glow/Tower/Tower2.Tower2")
      (`PrimitiveComponent.SetMaterial` _platformhigh 1 "/Game/Materials/Glow/Tower/Tower2.Tower2")
      (`PrimitiveComponent.SetMaterial` _platformhigh 3 "/Game/Materials/Glow/Tower/Tower2.Tower2")
      (`DestructibleComponent.ApplyRadiusDamage` _platformhigh 1000.0 (`SceneComponent.K2_GetComponentLocation` _platformhigh) 500.0 75000.0 true))))

(fn `UserConstructionScript`)