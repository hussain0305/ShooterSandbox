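; Grabbable actor that shrinks when grabbed, grows back when fired, and can take on projectile collision.
; Grab and fire events call Multi-prefixed events whose timelines lerp actor scale between the captured size and a tenth of it.
; Naming is inverted: Multi_Grow scales down and Multi_Shrink scales up.
; Projectile collision switches to a custom object type that blocks all channels except two ignored custom ones.
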(event `self.ApplyVisualChangesUponGrab`
  (`self.Multi_Grow`))

(event `Multi_Grow`
  (bind _output_get (set `self.LargeScale` (`self.GetActorScale3D`)))
  (set `self.SmallScale` (/ _output_get 10))
  (bind (_direction _scaledownfactor) (`Timeline|ScaleDown` :!via `PlayFromStart`)
    (:`Update`
      (`self.SetActorScale3D` (`KismetMathLibrary.VLerp` (`self.LargeScale`) (`self.SmallScale`) _scaledownfactor)))))

(event `self.ApplyVisualChangesUponFire`
  (`self.Multi_Shrink`))

(event `Multi_Shrink`
  (bind (_direction _scaleupfactor) (`Timeline|ScaleUp` :!via `PlayFromStart`)
    (:`Update`
      (`self.SetActorScale3D` (`KismetMathLibrary.VLerp` (`self.SmallScale`) (`self.LargeScale`) _scaleupfactor)))))

(event `self.BP_ApplyProjectileCollisionSettings`
  (bind _collisioncomponent (`self.CollisionComponent`))
  (`PrimitiveComponent.SetCollisionEnabled` _collisioncomponent "QueryAndPhysics")
  (`PrimitiveComponent.SetCollisionObjectType` _collisioncomponent "ECC_GameTraceChannel2")
  (`PrimitiveComponent.SetCollisionResponseToAllChannels` _collisioncomponent "ECR_Block")
  (`PrimitiveComponent.SetCollisionResponseToChannel` _collisioncomponent "ECC_GameTraceChannel3" "ECR_Ignore")
  (`PrimitiveComponent.SetCollisionResponseToChannel` _collisioncomponent "ECC_GameTraceChannel6" "ECR_Ignore"))

(fn `UserConstructionScript`)